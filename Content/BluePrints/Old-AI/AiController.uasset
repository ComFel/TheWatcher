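; AI controller for enemy characters that caches the possessed EnemyCharacter and starts its behavior tree.
; Walk/Patrol and Run/Chase events forward to the enemy's WalkPatrol and RunChase functions.
; The perception update event is empty; the logic that would write CanSeePlayer to the blackboard on sensing ControlledObject2 is disconnected.
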(event `self.AIPerception.OnTargetPerceptionUpdated`
  (params (Actor :type "Actor Object Reference") (Stimulus :type "AIStimulus Structure")))

(event `Walk/Patrol`
  (`/Game/BluePrints/Old-AI/EnemyCharacter.Walk/Patrol` (`self.Enemy`)))

(event `Run/Chase`
  (`/Game/BluePrints/Old-AI/EnemyCharacter.Run/Chase` (`self.Enemy`)))

(event `self.ReceivePossess`
  (params (PossessedPawn :type "Pawn Object Reference"))
  (bind _asenemy_character (cast `/Game/BluePrints/Old-AI/EnemyCharacter` PossessedPawn))
  (set `self.Enemy` _asenemy_character)
  (`self.RunBehaviorTree` "/Game/BluePrints/Old-AI/Enemy.Enemy"))

(fn `UserConstructionScript`)