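; AI controller for NPCs that seeds a blackboard and starts their behavior tree.
; On BeginPlay it scans PathPoint actors by their Mensaje tag, storing "Path1" and "Lejos" locations as the near (CercaPosition) and far (LejosPosition) positions.
; It stores the first ControlledObject found as the Enemy, then runs NPC_BehaviorTree after a short delay.
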(event `self.ReceiveBeginPlay`
  (bind _returnvalue (`AIBlueprintHelperLibrary.GetBlackboard` self))
  (`self.UseBlackboard` "/Game/BluePrints/NPC/NPC_Blackboard.NPC_Blackboard")
  (`|ExecutionSequence`
    (:`then_0`
      (bind _outactors (`GameplayStatics.GetAllActorsOfClass` "/Game/BluePrints/PathPoint_Blueprint.PathPoint_Blueprint_C"))
      (for _array_element _outactors
        (bind _aspath_point_blueprint (cast `/Game/BluePrints/PathPoint_Blueprint` _array_element))
        (bind _mensaje (`/Game/BluePrints/PathPoint_Blueprint.Mensaje` _aspath_point_blueprint))
        (if (`KismetStringLibrary.EqualEqual_StrStr` _mensaje (`self.Path1`))
          (`BlackboardComponent.SetValueAsVector` _returnvalue (`self.CercaPosition`) (`self.K2_GetActorLocation` _aspath_point_blueprint))
          (elif (`KismetStringLibrary.EqualEqual_StrStr` _mensaje (`self.Lejos`))
            (`BlackboardComponent.SetValueAsVector` _returnvalue (`self.LejosPosition`) (`self.K2_GetActorLocation` _aspath_point_blueprint))))))
    (:`then_1`
      (bind _outactors_2 (`GameplayStatics.GetAllActorsOfClass` "/Game/BluePrints/ControlledObject.ControlledObject_C"))
      (`BlackboardComponent.SetValueAsObject` (`AIBlueprintHelperLibrary.GetBlackboard` self) (`self.Enemy`) (`|GetArrayItem` _outactors_2))
      (`KismetSystemLibrary.Delay` 1.0)
      (`self.RunBehaviorTree` "/Game/BluePrints/NPC/NPC_BehaviorTree.NPC_BehaviorTree"))))

(fn `UserConstructionScript`)