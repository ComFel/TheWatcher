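; MoveToPath1 is a behavior tree task that walks an NPC to the location stored in its Path1 blackboard key.
; On execute it casts the owner to NPC_Controller and opens a Gate, which lets Tick issue AIMoveTo on the controlled pawn every frame.
; A successful move finishes the task and closes the Gate through CerrarPuerta; failed casts or moves never finish it.
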(event `self.ReceiveTick`
  (params (OwnerActor :type "Actor Object Reference") (DeltaSeconds :type "Float (single-precision)"))
  (`/Engine/EditorBlueprintResources/StandardMacros.Gate` true :!label _label
    (:`Exit`
      (`|AIMoveTo` (`Controller.K2_GetPawn` (stale `self.ReceiveExecute` _asnpc_controller)) (`BlackboardComponent.GetValueAsVector` (`AIBlueprintHelperLibrary.GetBlackboard` (stale `self.ReceiveExecute` _asnpc_controller)) (`self.Path 1`)) null 1.0
        (:`OnSuccess`
          (`self.FinishExecute` true)
          (`self.CerrarPuerta`))))))

(event `CerrarPuerta`
  (goto _label :!via `Close`))

(event `self.ReceiveExecute`
  (params (OwnerActor :type "Actor Object Reference"))
  (bind _asnpc_controller (cast `/Game/BluePrints/NPC/NPC_Controller` OwnerActor))
  (goto _label :!via `Open`))