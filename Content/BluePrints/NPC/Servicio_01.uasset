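; Behavior Tree service that keeps an NPC's blackboard updated with its position relative to its enemy and two stored locations.
; Each tick it writes the pawn's distance to the Enemy into DistanciaEnemigo and sets MoveToCerca when that distance is within Umbral.
; CheckLocation uses a tolerance-based NearlyEqual helper to flag whether the pawn is at CercaLocation (near) or LejosLocation (far).
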(event `self.ReceiveTick`
  (params (OwnerActor :type "Actor Object Reference") (DeltaSeconds :type "Float (single-precision)"))
  (bind _movetocerca (`self.MoveToCerca`))
  (bind _asnpc_controller (cast `/Game/BluePrints/NPC/NPC_Controller` OwnerActor))
  (bind _ascontrolled_object (cast `/Game/BluePrints/ControlledObject` (`BTFunctionLibrary.GetBlackboardValueAsObject` (`self.Enemy`))))
  (bind _returnvalue (`Actor.K2_GetActorLocation` (`Controller.K2_GetPawn` _asnpc_controller)))
  (set `self.Pawn Position` _returnvalue)
  (bind _returnvalue_2 (`KismetMathLibrary.VSize` (- (`Actor.K2_GetActorLocation` _ascontrolled_object) _returnvalue)))
  (`BTFunctionLibrary.SetBlackboardValueAsFloat` (`self.Distancia enemigo`) _returnvalue_2)
  (`self.Check Location`) ; Llama a check Location, ver recuadro de abajo
  (if (<= _returnvalue_2 (`self.Umbral`))
    (`BTFunctionLibrary.SetBlackboardValueAsBool` _movetocerca true)
    (else
      (`BTFunctionLibrary.SetBlackboardValueAsBool` _movetocerca))))

(event `Check Location`
  (bind _tolerancia (`self.Tolerancia`))
  ;[1 1 1] Establece variables del blackboard para saber donde se encuentra el NPC
  (bind _result (`self.Nearly Equal` (`self.Pawn Position`) (`BTFunctionLibrary.GetBlackboardValueAsVector` (`self.CercaLocation`)) _tolerancia))
  (bind _result_2 (`self.Nearly Equal` (`self.Pawn Position`) (`BTFunctionLibrary.GetBlackboardValueAsVector` (`self.LejosLocation`)) _tolerancia))
  (`BTFunctionLibrary.SetBlackboardValueAsBool` (`self.Estoy en cerca location`) _result)
  (`BTFunctionLibrary.SetBlackboardValueAsBool` (`self.Estoy en lejos location`) _result_2))

(fn `Nearly Equal`
  (params (`Vector 1` :type "Vector Structure") (`Vector 2` :type "Vector Structure") (Tolerancia :type "Float (double-precision)"))
  (returns (Result :type Boolean))
  (return (<= (`KismetMathLibrary.Abs` (`KismetMathLibrary.VSize` (- `Vector 1` `Vector 2`))) Tolerancia)))