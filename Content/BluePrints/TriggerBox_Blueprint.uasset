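; Trigger box Blueprint that tracks suspicious (SUS) ControlledObject2 actors inside its area.
; On BeginPlay it registers itself as the Area reference on MyGameMode.
; Begin overlap adds objects flagged SUS to ListaDeSUS, and end overlap removes any departing ControlledObject2 from that list.
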(event `self.ReceiveBeginPlay`
  ;[1 1 1] Guarda una referencia a la Trigger Box en el controlador
  (bind _asmy_game_mode (cast `/Game/BluePrints/MyGameMode` (`GameplayStatics.GetGameMode`)))
  (set `/Game/BluePrints/MyGameMode.Area` self _asmy_game_mode))

(event `self.CollisionComponent.OnComponentBeginOverlap`
  (params (OverlappedComponent :type "PrimitiveComponent Object Reference") (OtherActor :type "Actor Object Reference") (OtherComp :type "PrimitiveComponent Object Reference") (OtherBodyIndex :type Integer) (bFromSweep :type Boolean) (SweepResult :type "HitResult Structure (by ref)"))
  ;[1 1 1] Guarda una referencia onCollision al Controlled Object en caso de que si sea sospechoso
  (bind _ascontrolled_object_2 (cast `/Game/BluePrints/ControlledObject2` OtherActor))
  (if (`/Game/BluePrints/ControlledObject2.SUS` _ascontrolled_object_2)
    (`KismetArrayLibrary.Array_Add` (`self.ListaDeSUS`) _ascontrolled_object_2)))

(event `self.CollisionComponent.OnComponentEndOverlap`
  (params (OverlappedComponent :type "PrimitiveComponent Object Reference") (OtherActor :type "Actor Object Reference") (OtherComp :type "PrimitiveComponent Object Reference") (OtherBodyIndex :type Integer))
  ;[1 1 1] Elimina la referencia de la lista cuando el Controlled Object sale del área
  (bind _ascontrolled_object_2 (cast `/Game/BluePrints/ControlledObject2` OtherActor))
  (`KismetArrayLibrary.Array_RemoveItem` (`self.ListaDeSUS`) _ascontrolled_object_2))

(fn `UserConstructionScript`)